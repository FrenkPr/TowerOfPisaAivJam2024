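; BP_Plane is a short-lived flying plane hazard that damages any actor it overlaps, then destroys itself.
; On BeginPlay it randomizes its max fly speed through CharacterMovement and picks one of two materials for body and propeller.
; Tick spins the propeller mesh by a fixed, frame-rate-dependent step, and a delay destroys the plane if it hits nothing.
; The graph itself issues no movement input.
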(event EventBeginPlay
  (Variables|/Script/Engine.CharacterMovementComponent|SetMaxFlySpeed (Variables|Character|GetCharacterMovement) (Math|Random|RandomFloatinRange 6e+02 2.4e+03))
  (if (Math|Random|RandomBool)
    (Rendering|Material|SetMaterial (Variables|Default|Getaereo_aereo) 0 "/Game/Pisa/Models/Texture/M_Plane1.M_Plane1")
    (Rendering|Material|SetMaterial (Variables|Default|Getaereo_Elica) 0 "/Game/Pisa/Models/Texture/M_Plane1.M_Plane1")
    (else
      (Rendering|Material|SetMaterial (Variables|Default|Getaereo_aereo) 0 "/Game/Pisa/Models/Texture/M_Plane2.M_Plane2")
      (Rendering|Material|SetMaterial (Variables|Default|Getaereo_Elica) 0 "/Game/Pisa/Models/Texture/M_Plane2.M_Plane2")))
  (Utilities|FlowControl|Delay 8.0)
  (if (Utilities|IsValid self)
    (Actor|DestroyActor)))

(event Collision|EventActorBeginOverlap
  (params (OtherActor :type Actor%20Object%20Reference))
  (Game|Damage|ApplyDamage OtherActor 5.0 0 0)
  (Actor|DestroyActor))

(event EventTick
  (params (DeltaSeconds :type Float%20%28single-precision%29))
  (Transformation|AddLocalRotation (Variables|Default|Getaereo_Elica) "33.000000,0.000000,0.000000" false false))

(fn ConstructionScript)