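; Actor that periodically spawns a BP_Plane and flies it along its spline.
; On Tick, once a random cooldown elapses, it spawns the plane, passes it the spawner's danger position and restarts a timeline.
; The timeline moves the plane by distance along the spline, remapping rotation axes with a yaw offset to orient it.
; A single stored plane reference and timeline drive the movement, so only the latest plane is moved.
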(event EventBeginPlay
  (Variables|Default|SetCooldown (Math|Random|RandomFloatinRange 8.0 2e+01)))

(event EventTick
  (params (DeltaSeconds :type Float%20%28single-precision%29))
  (bind _spline (Variables|Default|GetSpline))
  (if (>= (- (Utilities|Time|GetTimeSeconds) (Variables|Default|GetLast%20Spawn)) (Variables|Default|GetCooldown))
    (bind _returnvalue (Game|SpawnActorfromClass "/Game/Pisa/BPs/BP_Plane.BP_Plane_C" (Transformation|GetWorldTransform (Variables|Default|GetDefaultSceneRoot)) "AlwaysSpawn" "MultiplyWithRoot" 0 0))
    (Variables|Default|SetLast%20Spawn (Utilities|Time|GetTimeSeconds))
    (Variables|Default|SetCooldown (Math|Random|RandomFloatinRange 8.0 2e+01))
    (Variables|/Game/Pisa/BPs/BP_Plane.BP_Plane_C|SetE_DangerPosition _returnvalue (Variables|Default|GetAirplaneDangerPosition))
    (bind _positiontrack (Timeline|Timeline PlayFromStart)
      (:Update
        (Utilities|IsValid _returnvalue
          (:Is%20Valid
            (Transformation|SetWorldTransform (Variables|/Script/Engine.Actor|GetRootComponent _returnvalue) (Math|Transform|MakeTransform (Spline|GetLocationatDistanceAlongSpline _spline (* _positiontrack (Spline|GetSplineLength _spline)) "World") (Math|Rotator|MakeRotator (* (.pitch (Spline|GetRotationatDistanceAlongSpline _spline (* _positiontrack (Spline|GetSplineLength _spline)) "World")) -1.0) (.roll (Spline|GetRotationatDistanceAlongSpline _spline (* _positiontrack (Spline|GetSplineLength _spline)) "World")) (- (.yaw (Spline|GetRotationatDistanceAlongSpline _spline (* _positiontrack (Spline|GetSplineLength _spline)) "World")) 9e+01)) "1.000000,1.000000,1.000000") false false)))))))

(fn ConstructionScript)