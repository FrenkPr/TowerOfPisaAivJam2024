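; BP_SideScrollMode is a side-scroller game mode that handles player respawning and keeps run counters.
; RespawnPlayer spawns a new actor of the player's class at the stored RespawnTransform, increments the death counter and has player controller 0 possess the new actor.
; A separate CollectiblesCounterIncrement event raises the collectibles count.
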(event Custom|Respawn%20Player
  (params (Player :type Character%20Object%20Reference))
  (bind _respawn_transform (Variables|Default|GetRespawn%20Transform))
  (bind _returnvalue (Game|SpawnActorfromClass (Utilities|GetClass Player) (Math|Transform|MakeTransform (.location _respawn_transform) (.rotation _respawn_transform) "1.000000,1.000000,1.000000") "Undefined" "SelectDefaultAtRuntime" 0 0))
  (CallFunction|DeathCounterIncrement)
  (Pawn|Possess (Game|GetPlayerController 0) _returnvalue))

(event Custom|Death%20Counter%20Increment
  ;[1 1 1] Death Counter set
  (bind _result (Math|Integer|IncrementInt (Variables|Default|GetCounter%20%20Death))
    (:%20%20
      (Variables|Default|SetCounter%20%20Death _result))))

(event Custom|Collectibles%20Counter%20Increment
  ;[1 1 1] Collectibles Counter set
  (bind _result (Math|Integer|IncrementInt (Variables|Default|GetCounter%20Collectibles))
    (:%20%20
      (Variables|Default|SetCounter%20Collectibles _result))))

(fn ConstructionScript
  (|CallParentFunction))