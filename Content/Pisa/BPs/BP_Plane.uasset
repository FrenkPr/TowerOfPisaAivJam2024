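; BP_Plane is a flying hazard for the Pisa tower game, with randomized speed, one of two random materials, a spinning propeller and an eight-second lifetime.
; Each tick it drives a HUD danger image in two distance stages from the player, clearing it after the closer warning or when destroyed.
; On overlap it damages the other actor, explodes, capsule-traces toward the tower to attach an impact decal, then destroys itself.
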(event Custom|RotateElica
  (Transformation|AddLocalRotation (Variables|Default|Getaereo_Elica) "33.000000,0.000000,0.000000" false false))

(event Custom|UpdateUIDangerImage
  (bind _returnvalue (Game|Player|GetPlayerPawn 0))
  (bind _self self)
  (bind _returnvalue_2 (Transformation|GetSquaredDistanceTo _self _returnvalue))
  (if (and (Utilities|IsValid self) (Variables|Default|GetUpdateUIDanger))
    (if (<= _returnvalue_2 2.5e+07)
      (Default|SetTextureAirplaneDangerImage (CallFunction|GetPlayerWBPHUD) (Variables|Default|GetE_DangerPosition) "NewEnumerator2")
      (Utilities|FlowControl|Delay 1.0)
      (Default|ClearTextureAirplaneDangerImage (CallFunction|GetPlayerWBPHUD) (Variables|Default|GetE_DangerPosition))
      (Variables|Default|SetUpdateUIDanger false)
      (elif (<= _returnvalue_2 5e+07)
        (Default|SetTextureAirplaneDangerImage (CallFunction|GetPlayerWBPHUD) (Variables|Default|GetE_DangerPosition) "NewEnumerator1")))))

(event EventBeginPlay
  (Variables|/Script/Engine.CharacterMovementComponent|SetMaxFlySpeed (Variables|Character|GetCharacterMovement) (Math|Random|RandomFloatinRange 6e+02 2.4e+03))
  (AddComponent|AddAudioComponent false)
  (if (Math|Random|RandomBool)
    (Rendering|Material|SetMaterial (Variables|Default|Getaereo_aereo) 0 "/Game/Pisa/Models/Texture/M_Plane1.M_Plane1")
    (Rendering|Material|SetMaterial (Variables|Default|Getaereo_Elica) 0 "/Game/Pisa/Models/Texture/M_Plane1.M_Plane1")
    (else
      (Rendering|Material|SetMaterial (Variables|Default|Getaereo_aereo) 0 "/Game/Pisa/Models/Texture/M_Plane2.M_Plane2")
      (Rendering|Material|SetMaterial (Variables|Default|Getaereo_Elica) 0 "/Game/Pisa/Models/Texture/M_Plane2.M_Plane2")))
  (Utilities|FlowControl|Delay 8.0)
  (if (Utilities|IsValid self)
    (Actor|DestroyActor)))

(event Collision|EventActorBeginOverlap
  (params (OtherActor :type Actor%20Object%20Reference))
  (bind _player (CallFunction|GetPlayerRef))
  (bind _aereo_elica (Variables|Default|Getaereo_Elica))
  (bind _returnvalue (Transformation|GetWorldLocation _aereo_elica))
  (bind _torredipisa_comb_torredipisa (Variables|/Game/Pisa/BPs/BP_PisaTower.BP_PisaTower_C|GetTorrediPisa_Comb_TorrediPisa _player))
  (bind _returnvalue_2 (Transformation|GetWorldLocation _torredipisa_comb_torredipisa))
  (Game|Damage|ApplyDamage OtherActor 5.0 0 0)
  (Effects|SpawnEmitteratLocation "/Game/StarterContent/Particles/P_Explosion.P_Explosion" _returnvalue "0, 0, 0" "10.000000,10.000000,10.000000")
  (Audio|PlaySound2D "/Game/Pisa/Sounds/387230__evanboyerman__explosion-var-2-closenear-mixed.387230__evanboyerman__explosion-var-2-closenear-mixed" 1.0 1.0 0.0 0 0)
  (bind _outhit (Collision|CapsuleTraceByChannel _returnvalue (Math|Vector|MakeVector (.x _returnvalue_2) (.y _returnvalue_2) (.Z (Math|Vector|BreakVector _returnvalue))) 5e+01 0.0 "TraceTypeQuery3" false 0 "None" true "(R=1.000000,G=0.000000,B=0.000000,A=1.000000)" "(R=0.000000,G=1.000000,B=0.000000,A=1.000000)" 3e+01))
  (Class|GameplayStatics|SpawnDecalAttached "/Game/Pisa/Models/Texture/PisaTower/M_PisaTowerDecal.M_PisaTowerDecal" "300.000000,300.000000,300.000000" (Variables|/Game/Pisa/BPs/BP_PisaTower.BP_PisaTower_C|GetTorrediPisa_Comb_TorrediPisa (CallFunction|GetPlayerRef)) "None" (* (+ (Math|Vector|VectorLength (.impactpoint _outhit)) 3e+01) (Math|Vector|Normalize (.impactpoint _outhit))) (Math|Conversions|RotationFromXVector (.impactnormal _outhit)) "KeepWorldPosition" 0.0)
  (Actor|DestroyActor))

(event EventTick
  (params (DeltaSeconds :type Float%20%28single-precision%29))
  (CallFunction|RotateElica)
  (CallFunction|UpdateUIDangerImage))

(event EventDestroyed
  (Default|ClearTextureAirplaneDangerImage (CallFunction|GetPlayerWBPHUD) (Variables|Default|GetE_DangerPosition)))

(fn ConstructionScript)