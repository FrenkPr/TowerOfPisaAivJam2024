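; Spawner actor that periodically launches a BP_Plane along its spline while active, tagging it with a danger position.
; Tick checks a randomized cooldown, then, if a paired opposite spawner is valid, waits for that spawner's plane to be gone plus an accumulated delay.
; A timeline moves the spawned plane along the spline, remapping pitch and roll and offsetting yaw to orient it.
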(event EventBeginPlay
  (Variables|Default|SetCooldown (Math|Random|RandomFloatinRange 8.0 16.0)))

(event EventTick
  (params (DeltaSeconds :type Float%20%28single-precision%29))
  (bind _spline (Variables|Default|GetSpline))
  (if (and (>= (- (Utilities|Time|GetTimeSeconds) (Variables|Default|GetLast%20Spawn)) (Variables|Default|GetCooldown)) (Variables|Default|GetIsActive))
    ;[1 1 1] Waiting for destroying airplane spawned to the opposite spawner.
    ; In the case the opposite spawner variable is not valid, will directly spawn the airplane after the cooldown
    (bind _oppositeairplanespawner (Variables|Default|GetOppositeAirplaneSpawner)
      (:then
        (Variables|BP_AirplanesSpawner_C|GetAirplaneSpawned _oppositeairplanespawner
          (:then)
          (:else
            (bind _output_get (Variables|Default|SetOppositeAirplaneDestroyedElapsedTime (+ (Variables|Default|GetOppositeAirplaneDestroyedElapsedTime) (Utilities|Time|GetWorldDeltaSeconds))))
            (if (>= _output_get (Variables|Default|GetOppositeAirplaneDestroyedTimer))
              (Variables|Default|SetOppositeAirplaneDestroyedElapsedTime 0.0)
              (bind _returnvalue (Game|SpawnActorfromClass "/Game/Pisa/BPs/BP_Plane.BP_Plane_C" (Transformation|GetWorldTransform (Variables|Default|GetDefaultSceneRoot)) "AlwaysSpawn" "MultiplyWithRoot" 0 0 :!label _label))
              (Variables|Default|SetAirplaneSpawned _returnvalue)
              (Variables|Default|SetLast%20Spawn (Utilities|Time|GetTimeSeconds))
              (Variables|Default|SetCooldown (Math|Random|RandomFloatinRange 8.0 16.0))
              (Variables|/Game/Pisa/BPs/BP_Plane.BP_Plane_C|SetE_DangerPosition (Variables|Default|GetAirplaneSpawned) (Variables|Default|GetAirplaneDangerPosition))
              (bind _positiontrack (Timeline|Timeline PlayFromStart)
                (:Update
                  (Utilities|IsValid (Variables|Default|GetAirplaneSpawned)
                    (:Is%20Valid
                      (Transformation|SetWorldTransform (Variables|/Script/Engine.Actor|GetRootComponent (Variables|Default|GetAirplaneSpawned)) (Math|Transform|MakeTransform (Spline|GetLocationatDistanceAlongSpline _spline (* _positiontrack (Spline|GetSplineLength _spline)) "World") (Math|Rotator|MakeRotator (* (.pitch (Spline|GetRotationatDistanceAlongSpline _spline (* _positiontrack (Spline|GetSplineLength _spline)) "World")) -1.0) (.roll (Spline|GetRotationatDistanceAlongSpline _spline (* _positiontrack (Spline|GetSplineLength _spline)) "World")) (- (.yaw (Spline|GetRotationatDistanceAlongSpline _spline (* _positiontrack (Spline|GetSplineLength _spline)) "World")) 9e+01)) "1.000000,1.000000,1.000000") false false)))))))))
      (:else
        (goto _label)))))

(fn ConstructionScript)